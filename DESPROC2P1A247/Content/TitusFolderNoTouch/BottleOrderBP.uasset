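; BottleOrderBP is a bottle actor that a player can pick up, using an item value and held-item flags on the player.
; CheckItem lets the pickup through when the player's Item is not positive, or when they hold neither a can nor chips.
; A successful pickup adds a fixed amount to Item, sets HasBottle and destroys the actor.
; The event graph is inactive, so CheckItem relies on an outside caller.
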(fn `checkItem`
  (params (Player :type "/Game/FirstPerson/Blueprints/BP_FirstPersonCharacter Object Reference"))
  (if (> (`/Game/FirstPerson/Blueprints/BP_FirstPersonCharacter.Item` Player) 0.0)
    (if (`/Game/FirstPerson/Blueprints/BP_FirstPersonCharacter.hasCan` Player)
      _
      (elif (not (`/Game/FirstPerson/Blueprints/BP_FirstPersonCharacter.hasChips` Player))
        (if (`/Game/FirstPerson/Blueprints/BP_FirstPersonCharacter.hasBottle` Player)
          _
          (else
            _))
        (set `/Game/FirstPerson/Blueprints/BP_FirstPersonCharacter.Item` (+ (`/Game/FirstPerson/Blueprints/BP_FirstPersonCharacter.Item` Player) 16.0) Player :!label _label)
        (set `/Game/FirstPerson/Blueprints/BP_FirstPersonCharacter.hasBottle` true Player)
        (`self.K2_DestroyActor`)))
    (else
      (goto _label))))

(fn `UserConstructionScript`
  (`parent.UserConstructionScript`))