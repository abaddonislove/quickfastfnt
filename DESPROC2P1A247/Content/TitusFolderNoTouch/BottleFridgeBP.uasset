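; BottleFridgeBP is an interactable fridge that loses one random can from its contents each time it is used.
; BeginPlay fills the Cans array with the fridge's static mesh components.
; Interact calls GetCan, which rerolls random indices until it finds a visible mesh, then PickUpCan hides it.
; The reroll has no exit for an empty fridge, so it loops endlessly once every can is hidden.
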(event `self.ReceiveBeginPlay`
  (`self.Array`))

(event `/Game/TitusFolderNoTouch/InteractionInterface.Interact`
  (bind _out (`self.getCan`))
  (`self.PickUp Can` _out))

(fn `Array`
  (set `self.Cans` (`|MakeArray` (`self.StaticMesh`) (`self.StaticMesh4`) (`self.StaticMesh14`) (`self.StaticMesh9`) (`self.StaticMesh31`) (`self.StaticMesh12`) (`self.StaticMesh17`) (`self.StaticMesh3`) (`self.StaticMesh16`) (`self.StaticMesh15`) (`self.StaticMesh24`) (`self.StaticMesh20`) (`self.StaticMesh22`) (`self.StaticMesh2`) (`self.StaticMesh1`) (`self.StaticMesh8`) (`self.StaticMesh34`) (`self.StaticMesh35`) (`self.StaticMesh36`) (`self.StaticMesh37`) (`self.StaticMesh38`) (`self.StaticMesh39`) (`self.StaticMesh40`) (`self.StaticMesh33`) (`self.StaticMesh28`) (`self.StaticMesh25`) (`self.StaticMesh30`) (`self.StaticMesh23`) (`self.StaticMesh26`) (`self.StaticMesh27`) (`self.StaticMesh29`) (`self.StaticMesh32`))))

(fn `getCan`
  (returns (Out :type "StaticMeshComponent Object Reference"))
  (bind _cans (`self.Cans`))
  (bind _output_get (set `self.Output` (`|GetArrayItem` _cans (`KismetMathLibrary.RandomInteger` (`KismetArrayLibrary.Array_Length` _cans))) :!label _label))
  (if (`SceneComponent.bVisible` _output_get)
    (return _output_get)
    (else
      (goto _label))))

(fn `PickUp Can`
  (params (worked :type "StaticMeshComponent Object Reference"))
  (if (`SceneComponent.bVisible` worked)
    (`SceneComponent.SetVisibility` worked false false)
    (else
      (`self.getCan`))))

(fn `UserConstructionScript`)