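; Shelf manager actor that builds a square storage grid of shelf cells and flags when the first-person character comes near.
; On BeginPlay, PopulateShelf spawns and stores ShelfCellBP actors, centered around world origin rather than the manager.
; Sphere overlap sets the character's ByShelf flag, which is never cleared here.
; GetClosestGridPosition looks unfinished: its loop tests the manager's location, returning either the first cell's position or zero.
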(event `self.ReceiveBeginPlay`
  (`self.Populate Shelf`))

(event `self.Sphere.OnComponentBeginOverlap`
  (params (OverlappedComponent :type "PrimitiveComponent Object Reference") (OtherActor :type "Actor Object Reference") (OtherComp :type "PrimitiveComponent Object Reference") (OtherBodyIndex :type Integer) (bFromSweep :type Boolean) (SweepResult :type "HitResult Structure (by ref)"))
  (bind _asbp_first_person_character (cast `/Game/FirstPerson/Blueprints/BP_FirstPersonCharacter` OtherActor))
  (set `/Game/FirstPerson/Blueprints/BP_FirstPersonCharacter.byShelf>` true _asbp_first_person_character))

(fn `GetClosestGridPosition`
  (params (InPos :type "Vector Structure"))
  (returns (OutPos :type "Vector Structure"))
  (locals (ClosestPos :type "Vector Structure") (ClosestDistance :type "Float (double-precision)"))
  (bind _returnvalue (`KismetMathLibrary.Vector_Distance` (`self.K2_GetActorLocation`) InPos))
  (bind _returnvalue_2 (`self.K2_GetActorLocation` (`|GetArrayItem` (`self.ItemArray`))))
  (set `local.ClosestPos` _returnvalue_2)
  (set `local.ClosestDistance` (`KismetMathLibrary.Vector_Distance` InPos _returnvalue_2))
  (for _ (`self.ItemArray`)
    (if (< _returnvalue (`local.ClosestDistance`))
      (set `local.ClosestPos` (0.0 0.0 0.0))
      (set `local.ClosestDistance` _returnvalue)))
  (return (`local.ClosestPos`)))

(fn `Populate Shelf`
  (locals (WorldOffset :type "Float (double-precision)"))
  (bind _shelfsize (`self.ShelfSize`))
  (bind _shelfsize_2 (`self.ShelfSize`))
  (bind _returnvalue (`KismetMathLibrary.FTrunc` (`local.WorldOffset`)))
  (`KismetArrayLibrary.Array_Clear` (`self.ItemArray`))
  (set `local.WorldOffset` (`KismetMathLibrary.Conv_IntToDouble` (- (/ (* (`self.StorageSize`) _shelfsize) 2) (/ _shelfsize 2))))
  (for _index (range (`self.StorageSize`))
    (for _index_2 (range (`self.StorageSize`))
      (bind _returnvalue_2 (`|SpawnActorFromClass` "/Game/TitusFolderNoTouch/ShelfCellBP.ShelfCellBP_C" (`KismetMathLibrary.MakeTransform` (`KismetMathLibrary.MakeVector` (`KismetMathLibrary.Conv_IntToDouble` (- (* _index_2 _shelfsize_2) _returnvalue)) (`KismetMathLibrary.Conv_IntToDouble` (- (* _shelfsize_2 _index) _returnvalue)))) "AlwaysSpawn" "MultiplyWithRoot" null null))
      (`KismetArrayLibrary.Array_Add` (`self.ItemArray`) _returnvalue_2))))

(fn `UserConstructionScript`)