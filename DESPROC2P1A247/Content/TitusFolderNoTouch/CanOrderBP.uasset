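; Grocery can display actor that the first-person player interacts with to take cans, with a prompt shown while they overlap its box.
; Construction builds a row-by-column grid of box slots, also spawning a GroceryItem at a random slot per iteration; BeginPlay spawns and attaches one at each slot.
; Interact adds to the player's Item, flags HasCan and destroys the display, unless a non-empty player holds a bottle or chips.
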(event `self.ReceiveBeginPlay`
  (for _array_element (`self.Cans`)
    (bind _returnvalue (`|SpawnActorFromClass` (`self.GroceryItem`) (`KismetMathLibrary.MakeTransform` (`SceneComponent.K2_GetComponentLocation` _array_element)) "Undefined" "MultiplyWithRoot" null null))
    (`self.K2_AttachToActor` _returnvalue self "None" "SnapToTarget" "SnapToTarget" "KeepRelative" true)))

(event `/Game/TitusFolderNoTouch/InteractionInterface.Interact`
  (bind _asbp_first_person_character (cast `/Game/FirstPerson/Blueprints/BP_FirstPersonCharacter` (`GameplayStatics.GetPlayerPawn` 0)))
  (`self.checkItem` _asbp_first_person_character))

(event `self.Box.OnComponentBeginOverlap`
  (params (OverlappedComponent :type "PrimitiveComponent Object Reference") (OtherActor :type "Actor Object Reference") (OtherComp :type "PrimitiveComponent Object Reference") (OtherBodyIndex :type Integer) (bFromSweep :type Boolean) (SweepResult :type "HitResult Structure (by ref)"))
  (cast `/Game/FirstPerson/Blueprints/BP_FirstPersonCharacter` OtherActor)
  (`SceneComponent.SetVisibility` (`self.Prompt`) true false))

(event `self.Box.OnComponentEndOverlap`
  (params (OverlappedComponent :type "PrimitiveComponent Object Reference") (OtherActor :type "Actor Object Reference") (OtherComp :type "PrimitiveComponent Object Reference") (OtherBodyIndex :type Integer))
  (cast `/Game/FirstPerson/Blueprints/BP_FirstPersonCharacter` OtherActor)
  (`SceneComponent.SetVisibility` (`self.Prompt`) false false))

(fn `Array`
  (`|SpawnActorFromClass` (`self.GroceryItem`) (`SceneComponent.K2_GetComponentToWorld` (`KismetArrayLibrary.Array_Random` (`self.Cans`))) "Undefined" "MultiplyWithRoot" null null))

(fn `checkItem`
  (params (Player :type "/Game/FirstPerson/Blueprints/BP_FirstPersonCharacter Object Reference"))
  (if (> (`/Game/FirstPerson/Blueprints/BP_FirstPersonCharacter.Item` Player) 0.0)
    (if (`/Game/FirstPerson/Blueprints/BP_FirstPersonCharacter.hasBottle` Player)
      _
      (elif (not (`/Game/FirstPerson/Blueprints/BP_FirstPersonCharacter.hasChips` Player))
        (if (`/Game/FirstPerson/Blueprints/BP_FirstPersonCharacter.hasCan` Player)
          _
          (else
            _))
        (set `/Game/FirstPerson/Blueprints/BP_FirstPersonCharacter.Item` (+ (`/Game/FirstPerson/Blueprints/BP_FirstPersonCharacter.Item` Player) 16.0) Player :!label _label)
        (set `/Game/FirstPerson/Blueprints/BP_FirstPersonCharacter.hasCan` true Player)
        (`self.K2_DestroyActor`)))
    (else
      (goto _label))))

(fn `getCan`
  (returns (Out :type "StaticMeshComponent Object Reference")))

(fn `PickUp Can`
  (params (worked :type "StaticMeshComponent Object Reference"))
  (if (`SceneComponent.bVisible` worked)
    (`SceneComponent.SetVisibility` worked false false)
    (else
      (`self.getCan`))))

(fn `UserConstructionScript`
  (for _index (range (+ (`self.Rows`) 1))
    (for _index_2 (range (+ (`self.Collumns`) 1))
      (bind _returnvalue (`AddComponent|NODE_AddBoxComponent-0` :`RelativeTransform` (`KismetMathLibrary.MakeTransform` (`KismetMathLibrary.MakeVector` (* _index_2 (`self.xDis`)) (* (`self.yDis`) _index) 0.17))))
      (`BoxComponent.SetBoxExtent` _returnvalue (10.0 10.0 10.0) true)
      (`KismetArrayLibrary.Array_Add` (`self.Cans`) _returnvalue)
      (`self.Array`))))