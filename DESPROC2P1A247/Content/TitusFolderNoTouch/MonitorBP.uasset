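; MonitorBP is an interactable monitor that manages a queue of AI actors waiting to pay, showing its widget while something overlaps its sphere.
; AddToQueue records actors and positions, returning the floor position for the front or the position of the actor ahead.
; Interact decrements each queued actor's LineIndex and sets the "Paid" blackboard key on any reaching -1.
; Tick uses delays to briefly toggle CanMove in a repeating pulse.
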(event `self.ReceiveTick`
  (params (DeltaSeconds :type "Float (single-precision)"))
  (bind _returnvalue (not (`self.CanMove`)))
  (`KismetSystemLibrary.Delay` 1.0)
  (set `self.CanMove` _returnvalue)
  (`KismetSystemLibrary.Delay` 0.2)
  (set `self.CanMove` _returnvalue))

(event `self.Sphere.OnComponentBeginOverlap`
  (params (OverlappedComponent :type "PrimitiveComponent Object Reference") (OtherActor :type "Actor Object Reference") (OtherComp :type "PrimitiveComponent Object Reference") (OtherBodyIndex :type Integer) (bFromSweep :type Boolean) (SweepResult :type "HitResult Structure (by ref)"))
  (`SceneComponent.SetVisibility` (`self.Widget`) true false))

(event `self.Sphere.OnComponentEndOverlap`
  (params (OverlappedComponent :type "PrimitiveComponent Object Reference") (OtherActor :type "Actor Object Reference") (OtherComp :type "PrimitiveComponent Object Reference") (OtherBodyIndex :type Integer))
  (`SceneComponent.SetVisibility` (`self.Widget`) false false))

(event `/Game/TitusFolderNoTouch/InteractionInterface.Interact`
  (params (actor :type "Actor Object Reference"))
  (for _array_element (`self.QueueActors`)
    (bind _lineindex (`/Game/TitusFolderNoTouch/BPCustomerAdult.LineIndex` _array_element))
    (set `/Game/TitusFolderNoTouch/BPCustomerAdult.LineIndex` (- _lineindex 1) _array_element)
    (if (== _lineindex -1)
      (`BlackboardComponent.SetValueAsBool` (`AIBlueprintHelperLibrary.GetBlackboard` _array_element) "Paid" true))))

(fn `Add to Queue`
  (params (QueueActorName :type String) (ActorLocation :type "Vector Structure") (QueueActor :type "/Game/TitusFolderNoTouch/BPCustomerAdult Object Reference"))
  (returns (QueueLocation :type "Vector Structure") (QueuePosition :type Integer) (AtBeginning :type Boolean))
  (bind _floorposition (`self.FloorPosition`))
  (bind _returnvalue (`KismetArrayLibrary.Array_Find` (`self.QueueActorNames`) QueueActorName))
  ;[1 1 1] Already Registered
  (if (`KismetArrayLibrary.Array_IsValidIndex` (`self.QueueActorNames`) _returnvalue)
    ;[1 1 1] Update Location
    (`KismetArrayLibrary.Array_Set` (`self.QueueActorPositions`) _returnvalue ActorLocation)
    (set `self.NumberInQueue` _returnvalue)
    (else
      (`KismetArrayLibrary.Array_Add` (`self.QueueActors`) QueueActor)
      ;[1 1 1] Newly registered
      (bind _returnvalue_2 (`KismetArrayLibrary.Array_Add` (`self.QueueActorNames`)))
      (`KismetArrayLibrary.Array_Add` (`self.QueueActorPositions`) ActorLocation)
      (set `self.NumberInQueue` _returnvalue_2)))
  ;[1 1 1] Front Position?
  (if (== (`self.NumberInQueue`) 0)
    ;[1 1 1] Front position, Location changed to Front Position
    (`KismetArrayLibrary.Array_Set` (`self.QueueActorPositions`) 0 _floorposition)
    (return _floorposition 0 true)
    (else
      ;[1 1 1] Get position of actor in front of me in queue. Not in Front. Position in queue returned
      (set `self.FloorPosition` (`|GetArrayItem` (`self.QueueActorPositions`) (- (`self.NumberInQueue`) 1)))
      (return (`self.FloorPosition`) (`self.NumberInQueue`) false))))

(fn `UpdateIndex`)

(fn `UserConstructionScript`)