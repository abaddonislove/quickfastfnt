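; Store shelf actor that the player stocks with bottles, cans or chips and that adult customers take items from.
; When the player interacts with items left, it adds a mesh component in the next eight-column grid slot, computed from CurrentIndex, and sets its mesh by item type.
; An empty-handed player clears the last slot, while an adult customer receives that mesh first.
; The overlap logic and GenerateRows grid builder are unused.
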(event `self.ReceiveBeginPlay`
  (`self.Array`))

(event `/Game/TitusFolderNoTouch/InteractionInterface.Interact`
  (params (actor :type "Actor Object Reference"))
  (bind _heldobjects (`self.HeldObjects`))
  (bind _heldobjects_2 (`self.HeldObjects`))
  (bind _asbp_first_person_character (cast `/Game/FirstPerson/Blueprints/BP_FirstPersonCharacter` actor)
    (:`then`
      (`/Game/FirstPerson/Blueprints/BP_FirstPersonCharacter.RemoveItemFromBox` _asbp_first_person_character)
      (bind _item (`/Game/FirstPerson/Blueprints/BP_FirstPersonCharacter.Item` _asbp_first_person_character))
      (if (> _item 0.0)
        (bind _out (`self.Get First Invisible Static Mesh`))
        (`self.applyNewMeshMeshToInvisible` _asbp_first_person_character _out)
        (`self.makeMeshVisible` _out)
        (set `/Game/FirstPerson/Blueprints/BP_FirstPersonCharacter.Item` (- _item 1.0) _asbp_first_person_character)
        (else
          (`self.RemoveLastIndex` (`|GetArrayItem` _heldobjects (`KismetArrayLibrary.Array_LastIndex` _heldobjects)))
          (set `self.CurrentIndex` (- (`self.CurrentIndex`) 1))
          (`KismetSystemLibrary.PrintString` "removing"))))
    (:`CastFailed`
      (bind _meshtype (`self.SetMeshType`))
      (bind _asbpcustomer_adult (cast `/Game/TitusFolderNoTouch/BPCustomerAdult` actor))
      (`/Game/TitusFolderNoTouch/BPCustomerAdult.GenerateAndSetObjectMesh` _asbpcustomer_adult _meshtype)
      (`self.RemoveLastIndex` (`|GetArrayItem` _heldobjects_2 (`KismetArrayLibrary.Array_LastIndex` _heldobjects_2)))
      (set `self.CurrentIndex` (- (`self.CurrentIndex`) 1)))))

(event `self.Box.OnComponentBeginOverlap`
  (params (OverlappedComponent :type "PrimitiveComponent Object Reference") (OtherActor :type "Actor Object Reference") (OtherComp :type "PrimitiveComponent Object Reference") (OtherBodyIndex :type Integer) (bFromSweep :type Boolean) (SweepResult :type "HitResult Structure (by ref)")))

(fn `applyNewMeshMeshToInvisible`
  (params (Player :type "/Game/FirstPerson/Blueprints/BP_FirstPersonCharacter Object Reference") (CurrentStaticMesh :type "StaticMeshComponent Object Reference"))
  (if (> (`/Game/FirstPerson/Blueprints/BP_FirstPersonCharacter.Item` Player) 0.0)
    ;[1 1 1] Setting Mesh to Bottle
    (if (`/Game/FirstPerson/Blueprints/BP_FirstPersonCharacter.hasBottle` Player)
      (`StaticMeshComponent.SetStaticMesh` CurrentStaticMesh "/Game/ConvenienceStore/TestModules/BuildingBlocks/SodaBottle_Item.SodaBottle_Item")
      (else
        ;[1 1 1] Setting Mesh to Can
        (if (`/Game/FirstPerson/Blueprints/BP_FirstPersonCharacter.hasCan` Player)
          (`StaticMeshComponent.SetStaticMesh` CurrentStaticMesh "/Game/ConvenienceStore/TestModules/BuildingBlocks/Can_Item.Can_Item")
          (else
            ;[1 1 1] Setting Mesh to Chip
            (if (`/Game/FirstPerson/Blueprints/BP_FirstPersonCharacter.hasChips` Player)
              (`StaticMeshComponent.SetStaticMesh` CurrentStaticMesh "/Game/ConvenienceStore/TestModules/BuildingBlocks/Chip_Item.Chip_Item"))))))))

(fn `Array`
  (set `self.HeldObjects` (`|MakeArray` null null null null null null null null null null null null null null null null null null null null null null null null null null null null null null null null :!type "StaticMeshComponent Object Reference")))

(fn `Generate Rows`
  ;[1 1 1] Calculating Row Position
  (for _index (range (`self.Rows`))
    ;[1 1 1] Calculating Column Position
    (for _index_2 (range (`self.Columns`))
      (bind _returnvalue (`AddComponent|NODE_AddStaticMeshComponent-0` :`bManualAttachment` true :`RelativeTransform` (`KismetMathLibrary.Conv_VectorToTransform` (`KismetMathLibrary.MakeVector` (+ (* _index_2 (/ 162 (`self.Columns`))) -59.0) 0.0 (+ (* _index -37.0) 51.0)))))
      (`SceneComponent.K2_AttachToComponent` _returnvalue (`self.Box`) "None" "KeepRelative" "KeepRelative" "KeepWorld" true)
      (`PrimitiveComponent.SetCollisionEnabled` _returnvalue "NoCollision")
      (`KismetArrayLibrary.Array_Add` (`self.HeldObjects`) _returnvalue))))

(fn `Get First Invisible Static Mesh`
  (returns (Out :type "StaticMeshComponent Object Reference"))
  (bind _returnvalue (`AddComponent|NODE_AddStaticMeshComponent-1` :`bManualAttachment` true :`RelativeTransform` (`KismetMathLibrary.Conv_VectorToTransform` (`KismetMathLibrary.MakeVector` (`KismetMathLibrary.Conv_IntToDouble` (- (* (- (`self.CurrentIndex`) (* (/ (`self.CurrentIndex`) 8) 8)) 21.0) 75)) 0.0 (`KismetMathLibrary.Conv_IntToDouble` (+ (* (/ (`self.CurrentIndex`) 8) -37) 51))))))
  (`SceneComponent.K2_AttachToComponent` _returnvalue (`self.Box`) "None" "KeepRelative" "KeepRelative" "KeepWorld" true)
  (`KismetArrayLibrary.Array_Add` (`self.HeldObjects`) _returnvalue)
  (set `self.CurrentIndex` (+ (`self.CurrentIndex`) 1))
  (return _returnvalue))

(fn `makeMeshVisible`
  (params (worked :type "StaticMeshComponent Object Reference"))
  (if (not (`SceneComponent.bVisible` worked))
    (`SceneComponent.SetVisibility` worked true false)))

(fn `RemoveLastIndex`
  (params (`Static mesh` :type "StaticMeshComponent Object Reference"))
  (`StaticMeshComponent.SetStaticMesh` `Static mesh` null)
  (`KismetArrayLibrary.Array_RemoveItem` (`self.HeldObjects`) `Static mesh`))

(fn `SetMeshType`
  (returns (MeshType :type "StaticMesh Object Reference"))
  (bind _heldobjects (`self.HeldObjects`))
  (return (`StaticMeshComponent.StaticMesh` (`|GetArrayItem` _heldobjects (`KismetArrayLibrary.Array_LastIndex` _heldobjects)))))

(fn `UserConstructionScript`)