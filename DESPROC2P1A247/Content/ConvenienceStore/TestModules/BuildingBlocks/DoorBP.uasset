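; Interactable double door Blueprint from the ConvenienceStore test modules that alternates between open and closed on each Interact call.
; A FlipFlop calls OpenDoor or CloseDoor, which instantly rotate the two leaves in opposite directions or back to zero and set the Open flag.
; Overlap events on component R show a Widget when the first-person character enters and hide it when any actor leaves.
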(event `/Game/TitusFolderNoTouch/InteractionInterface.Interact`
  (`/Engine/EditorBlueprintResources/StandardMacros.FlipFlop`
    (:`A`
      (`self.OpenDoor`))
    (:`B`
      (`self.CloseDoor`))))

(event `self.r.OnComponentBeginOverlap`
  (params (OverlappedComponent :type "PrimitiveComponent Object Reference") (OtherActor :type "Actor Object Reference") (OtherComp :type "PrimitiveComponent Object Reference") (OtherBodyIndex :type Integer) (bFromSweep :type Boolean) (SweepResult :type "HitResult Structure (by ref)"))
  (cast `/Game/FirstPerson/Blueprints/BP_FirstPersonCharacter` OtherActor)
  (`SceneComponent.SetVisibility` (`self.Widget`) true false))

(event `self.r.OnComponentEndOverlap`
  (params (OverlappedComponent :type "PrimitiveComponent Object Reference") (OtherActor :type "Actor Object Reference") (OtherComp :type "PrimitiveComponent Object Reference") (OtherBodyIndex :type Integer))
  (`SceneComponent.SetVisibility` (`self.Widget`) false false))

(fn `CloseDoor`
  (`SceneComponent.K2_SetRelativeRotation` :`self` (`self.Door`))
  (`SceneComponent.K2_SetRelativeRotation` :`self` (`self.Door1`))
  (set `self.Open` false))

(fn `OpenDoor`
  (`SceneComponent.K2_SetRelativeRotation` (`self.Door`) (struct :`Yaw` -90.0) false false)
  (`SceneComponent.K2_SetRelativeRotation` (`self.Door1`) (struct :`Yaw` 90.0) false false)
  (set `self.Open` true))

(fn `UserConstructionScript`)