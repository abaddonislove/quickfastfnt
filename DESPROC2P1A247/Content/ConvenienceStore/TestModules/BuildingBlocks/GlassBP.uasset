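; Glass window building block for the convenience store that can start dirty and be cleaned by the player.
; On BeginPlay, a random roll against Chance swaps the clean Window mesh for DirtyWindow and sets IsDirty.
; A sphere overlap shows the interaction Widget to the first-person character only while dirty.
; Interact restores the clean window, hides the widget and deducts player Energy, without checking IsDirty.
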(event `self.ReceiveBeginPlay`
  (`self.Dirty?`)
  (bind _asbp_first_person_character (cast `/Game/FirstPerson/Blueprints/BP_FirstPersonCharacter` (`GameplayStatics.GetPlayerPawn` 0)))
  (set `self.playerref` _asbp_first_person_character))

(event `/Game/TitusFolderNoTouch/InteractionInterface.Interact`
  (bind _playerref (`self.playerref`))
  (`SceneComponent.SetVisibility` (`self.Window`) true false)
  (`SceneComponent.SetVisibility` (`self.DirtyWindow`) false false)
  (`KismetSystemLibrary.PrintText` "Hello")
  (set `self.isDirty` false)
  (`SceneComponent.SetVisibility` (`self.Widget`) false false)
  (bind _output_get (set `/Game/FirstPerson/Blueprints/BP_FirstPersonCharacter.Energy` (- (`/Game/FirstPerson/Blueprints/BP_FirstPersonCharacter.Energy` _playerref) 10.0) _playerref))
  (`KismetSystemLibrary.PrintString` (`KismetStringLibrary.Conv_DoubleToString` _output_get)))

(event `self.Sphere.OnComponentBeginOverlap`
  (params (OverlappedComponent :type "PrimitiveComponent Object Reference") (OtherActor :type "Actor Object Reference") (OtherComp :type "PrimitiveComponent Object Reference") (OtherBodyIndex :type Integer) (bFromSweep :type Boolean) (SweepResult :type "HitResult Structure (by ref)"))
  (cast `/Game/FirstPerson/Blueprints/BP_FirstPersonCharacter` OtherActor)
  (if (`self.isDirty`)
    (`SceneComponent.SetVisibility` (`self.Widget`) true false)))

(event `self.Sphere.OnComponentEndOverlap`
  (params (OverlappedComponent :type "PrimitiveComponent Object Reference") (OtherActor :type "Actor Object Reference") (OtherComp :type "PrimitiveComponent Object Reference") (OtherBodyIndex :type Integer))
  (`SceneComponent.SetVisibility` (`self.Widget`) false false))

(fn `Dirty?`
  (if (<= (`KismetMathLibrary.RandomIntegerInRange` 0 99) (`self.chance`))
    (`SceneComponent.SetVisibility` (`self.DirtyWindow`) true false)
    (`SceneComponent.SetVisibility` (`self.Window`) false false)
    (set `self.isDirty` true)))

(fn `UserConstructionScript`)