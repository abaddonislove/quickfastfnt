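; BP_MerchBox is an interactable merchandise box that fills itself with a grid of product meshes and tells the player what it holds.
; On BeginPlay, PhysicsHandleSetUp adds collision-free static mesh components in rows and columns, storing them in StaticMeshes.
; Interact sets the first-person character's Item to that count and flags bottle, chips or can by substring-matching the mesh asset's name.
; DeductFromArray removes one mesh but is only called from unconnected test nodes.
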(event `self.ReceiveBeginPlay`
  (`self.PhysicsHandleSetUp`))

(event `self.ReceiveTick`
  (params (DeltaSeconds :type "Float (single-precision)")))

(event `/Game/TitusFolderNoTouch/InteractionInterface.Interact`
  (params (actor :type "Actor Object Reference"))
  (bind _asbp_first_person_character (cast `/Game/FirstPerson/Blueprints/BP_FirstPersonCharacter` (`GameplayStatics.GetPlayerPawn` 0)))
  (`self.SetHeldItem` _asbp_first_person_character))

(fn `DeductFromArray`
  (bind _staticmeshes (`self.StaticMeshes`))
  (`ActorComponent.K2_DestroyComponent` (`|GetArrayItem` (`self.StaticMeshes`)))
  (`KismetArrayLibrary.Array_RemoveItem` _staticmeshes (`|GetArrayItem` _staticmeshes)))

(fn `PhysicsHandleSetUp`
  ;[1 1 1] Calculating Row Position
  (for _index (range (`self.Rows`))
    ;[1 1 1] Calculating Column Position
    (for _index_2 (range (`self.Columns`))
      ;[1 1 1] Making Physics Handle Component and Storing Array
      (bind _returnvalue (`AddComponent|NODE_AddStaticMeshComponent-0` :`bManualAttachment` true :`RelativeTransform` (`KismetMathLibrary.Conv_VectorToTransform` (`KismetMathLibrary.MakeVector` (+ (* _index (/ (`self.Width`) (`self.Rows`))) 10.0) (+ (* _index_2 (/ (`self.Height`) (`self.Columns`))) 10.0) 5.0))))
      (`SceneComponent.K2_AttachToComponent` _returnvalue (`self.Box`) "None" "KeepRelative" "KeepRelative" "KeepWorld" true)
      (`StaticMeshComponent.SetStaticMesh` _returnvalue (`self.MeshAsset`))
      (`PrimitiveComponent.SetCollisionEnabled` _returnvalue "NoCollision")
      (`KismetArrayLibrary.Array_Add` (`self.StaticMeshes`) _returnvalue))))

(fn `SetHeldItem`
  (params (Player :type "/Game/FirstPerson/Blueprints/BP_FirstPersonCharacter Object Reference"))
  (set `/Game/FirstPerson/Blueprints/BP_FirstPersonCharacter.Item` (`KismetMathLibrary.Conv_IntToDouble` (`KismetArrayLibrary.Array_Length` (`self.StaticMeshes`))) Player)
  (if (`KismetStringLibrary.Contains` (`KismetSystemLibrary.GetObjectName` (`self.MeshAsset`)) "bottle")
    (set `/Game/FirstPerson/Blueprints/BP_FirstPersonCharacter.hasBottle` true Player)
    (`KismetSystemLibrary.PrintString` "bottle")
    (elif (`KismetStringLibrary.Contains` (`KismetSystemLibrary.GetObjectName` (`self.MeshAsset`)) "chip")
      (set `/Game/FirstPerson/Blueprints/BP_FirstPersonCharacter.hasChips` true Player)
      (`KismetSystemLibrary.PrintString` "chips")
      (elif (`KismetStringLibrary.Contains` (`KismetSystemLibrary.GetObjectName` (`self.MeshAsset`)) "can")
        (set `/Game/FirstPerson/Blueprints/BP_FirstPersonCharacter.hasCan` true Player)
        (`KismetSystemLibrary.PrintString` "can")))))

(fn `UserConstructionScript`)